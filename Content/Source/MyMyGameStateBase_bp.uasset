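; GameState Blueprint that runs the on-screen dialogue flow and opens or closes the inventory widget.
; A DialogueSystem is searched by type and advanced on update unless options are showing; its callbacks swap or cancel widgets.
; ChangeWidget creates a plain or option dialogue widget by name, and content reaches it through the UpdateWidget interface.
; Option and inventory widgets enable the first-person character's mouse cursor, which is disabled when they clear.
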(event `self.ReceiveBeginPlay`
  ;[1 1 1] WidgetInitialization
  (set `self.HasDialogue` false)
  (set `self.HasOption` false))

(event `StartADialogue`
  (params (Type :type String) (Widget :type String))
  ;[1 1 1] StartADialogue
  (`self.CancelDialogue`)
  (`DialogueSystem.Search` (`self.DialogueSystem`) Type)
  (`self.ChangeWidget` Widget)
  (`DialogueSystem.Update` (`self.DialogueSystem`))
  (set `self.HasDialogue` true))

(event `UpdateDialogue`
  ;[1 1 1] UpdateDialogue
  (if (`self.HasDialogue`)
    (if (not (`self.HasOption`))
      (`DialogueSystem.Update` (`self.DialogueSystem`)))))

(event `PrintTest`
  (params (NewParam :type String) (NewParam2 :type "Array of String") (NewParam3 :type "Array of String"))
  ;[1 1 1] PrintTest
  (`KismetSystemLibrary.PrintString` "!!!!!!!!!")
  (`KismetSystemLibrary.PrintString` NewParam)
  (for (_array_element _array_index) NewParam2
    (`KismetSystemLibrary.PrintString` (`KismetStringLibrary.Concat_StrStr` _array_element (`|GetArrayItem` NewParam3 _array_index)))))

(event `self.DialogueSystem.UpdateWidget`
  (params (widgetName :type String) (updateContent :type "MyInterpStruct Structure"))
  (bind _currentwidget (`self.CurrentWidget`))
  ;[1 1 1] CallByC++DialogueWhenChange
  (if (not (or (`KismetStringLibrary.EqualEqual_StrStr` widgetName) (`KismetStringLibrary.EqualEqual_StrStr` widgetName (`self.CurrentWidgetName`))))
    (`self.ChangeWidget` widgetName)
    (`/Engine/EditorBlueprintResources/StandardMacros.IsValid` _currentwidget
      (:`Is Valid`
        _)))
  (if (`KismetSystemLibrary.DoesImplementInterface` _currentwidget "/Game/Source/Dialog/UpdateWidget.UpdateWidget_C")
    (message `/Game/Source/Dialog/UpdateWidget.UpdateWidget` _currentwidget updateContent_key updateContent_value)))

(event `CancelDialogue`
  (bind _currentwidget (`self.CurrentWidget`))
  ;[1 1 1] RemoveDialogueFromViewport
  (`/Engine/EditorBlueprintResources/StandardMacros.IsValid` _currentwidget :!label _label
    (:`Is Valid`
      (`Widget.RemoveFromParent` _currentwidget)
      (set `self.CurrentWidgetName` "")
      (set `self.CurrentWidget` null)
      (`self.ClearHasOption`)
      (set `self.HasDialogue` false))))

(event `self.DialogueSystem.Cancle`
  ;[1 1 1] RemoveDialogueFromViewport
  (goto _label))

(event `OpenInventory`
  (`KismetSystemLibrary.PrintString` "Open!!!")
  (bind _returnvalue (`|CreateWidget` "/Game/Source/Item/Inventory.Inventory_C" (`GameplayStatics.GetPlayerController` 0)))
  (bind _output_get (set `self.InventoryWidget` _returnvalue))
  (`UserWidget.AddToViewport` _output_get 0)
  (set `/Game/Source/Item/Inventory.MenuVisibility` "Visible" _output_get)
  (set `self.HasInventory` true)
  (bind _asfirst_person_character (cast `/Game/FirstPersonCPP/Blueprints/FirstPersonCharacter` (`GameplayStatics.GetPlayerCharacter` 0)))
  (`/Game/FirstPersonCPP/Blueprints/FirstPersonCharacter.EnableMouseCursor` _asfirst_person_character))

(event `AfterCloseInventory`
  (`KismetSystemLibrary.PrintString` "CloseOut")
  (`Widget.RemoveFromParent` (`self.InventoryWidget`))
  (set `self.InventoryWidget` null)
  (set `self.HasInventory` false)
  (bind _asfirst_person_character (cast `/Game/FirstPersonCPP/Blueprints/FirstPersonCharacter` (`GameplayStatics.GetPlayerCharacter` 0)))
  (`/Game/FirstPersonCPP/Blueprints/FirstPersonCharacter.DisableMouseCursor` _asfirst_person_character))

(fn `ChangeWidget`
  (params (WidgetName :type String))
  (bind _returnvalue (`GameplayStatics.GetPlayerController` 0))
  (bind _currentwidget (`self.CurrentWidget`))
  (`self.ClearHasOption`)
  (`/Engine/EditorBlueprintResources/StandardMacros.IsValid` _currentwidget
    (:`Is Valid`
      (`Widget.RemoveFromParent` _currentwidget))
    (:`Is Not Valid`
      _))
  (switch `string` (`KismetStringLibrary.ToLower` WidgetName)
    (:`Default`
      (bind _returnvalue_2 (`|CreateWidget` "/Game/Source/Dialog/DialogueWidget.DialogueWidget_C" _returnvalue :!label _label))
      (`UserWidget.AddToViewport` _returnvalue_2 0)
      (set `self.CurrentWidget` _returnvalue_2))
    (:`dialogue`
      (goto _label))
    (:`option`
      (set `self.HasOption` true)
      (bind _returnvalue_3 (`|CreateWidget` "/Game/Source/Dialog/DialogueWidgetOptions.DialogueWidgetOptions_C" _returnvalue))
      (`UserWidget.AddToViewport` _returnvalue_3 0)
      (set `self.CurrentWidget` _returnvalue_3)
      (bind _asfirst_person_character (cast `/Game/FirstPersonCPP/Blueprints/FirstPersonCharacter` (`GameplayStatics.GetPlayerCharacter` 0))
        (:`then`
          (`/Game/FirstPersonCPP/Blueprints/FirstPersonCharacter.EnableMouseCursor` _asfirst_person_character)
          (`KismetSystemLibrary.PrintString` "HasOption" true true (struct :`R` 0.959955 :`B` 1.0 :`A` 1.0)))
        (:`CastFailed`
          _))))
  (set `self.CurrentWidgetName` WidgetName))

(fn `ClearHasOption`
  (if (`self.HasOption`)
    (bind _asfirst_person_character (cast `/Game/FirstPersonCPP/Blueprints/FirstPersonCharacter` (`GameplayStatics.GetPlayerCharacter` 0)))
    (`/Game/FirstPersonCPP/Blueprints/FirstPersonCharacter.DisableMouseCursor` _asfirst_person_character)
    (set `self.HasOption` false)))

(fn `UserConstructionScript`)