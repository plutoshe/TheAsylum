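; BP_WorldCapture is a map-system actor that frames a world area for an orthographic scene capture, bounded by UpperLeft and LowerRight actors.
; When both references are valid, the construction script centers the actor between them in XY, keeping its Z.
; It then sets the capture's OrthoWidth to the larger X or Y separation.
; All logic runs at construction, and the event graph is empty.
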(fn `UserConstructionScript`
  (bind (_returnvalue_x _returnvalue_y _returnvalue_z) (`KismetMathLibrary.BreakVector` (`self.K2_GetActorLocation`)))
  (bind _upperleft (`self.UpperLeft`))
  (bind _lowerright (`self.LowerRight`))
  (bind (_returnvalue_x_2 _returnvalue_y_2) (`KismetMathLibrary.BreakVector` (`self.K2_GetActorLocation` (`self.UpperLeft`))))
  (bind (_returnvalue_x_3 _returnvalue_y_3) (`KismetMathLibrary.BreakVector` (`self.K2_GetActorLocation` (`self.LowerRight`))))
  (bind (_returnvalue_x_4 _returnvalue_y_4) (`KismetMathLibrary.BreakVector` (/ (+ (`self.K2_GetActorLocation` _upperleft) (`self.K2_GetActorLocation` _lowerright)) 2.0)))
  (`/Engine/EditorBlueprintResources/StandardMacros.IsValid` _upperleft
    (:`Is Valid`
      (`/Engine/EditorBlueprintResources/StandardMacros.IsValid` _lowerright
        (:`Is Valid`
          (`self.K2_SetActorLocation` (`KismetMathLibrary.MakeVector` _returnvalue_x_4 _returnvalue_y_4 _returnvalue_z) false true)
          (set `SceneCaptureComponent2D.OrthoWidth` (`KismetMathLibrary.FMax` (`KismetMathLibrary.Abs` (- _returnvalue_x_2 _returnvalue_x_3)) (`KismetMathLibrary.Abs` (- _returnvalue_y_2 _returnvalue_y_3))) (`self.SceneCapture`)))))))