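; Blueprint component that drives a world map widget showing the player's position within a rectangular area bounded by UpperLeft and LowerRight actors.
; Initialization creates W_main, caches its map widget and player marker size, then adds it to the viewport with the map hidden, toggleable via ToggleVisibility.
; Each tick it normalizes player location against those bounds, swaps X/Y into widget space and moves the centered marker by render translation.
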(event `Initialization`
  (params (Player :type "Character Object Reference"))
  (bind _mapref (`self.MapRef`))
  (`/Engine/EditorBlueprintResources/StandardMacros.IsValid` Player
    (:`Is Valid`
      (set `self.Player` Player)
      (bind _returnvalue (`|CreateWidget` "/Game/Source/MapSystem/Widgets/W_main.W_main_C"))
      (bind _output_get (set `self.WMainRef` _returnvalue))
      (bind _output_get_2 (set `self.MapRef` (`/Game/Source/MapSystem/Widgets/W_main.W_WorldMap` _output_get)))
      (`/Game/Source/MapSystem/Widgets/W_WorldMap.Initialization` _output_get_2 self)
      (set `self.OriginalPlayerSize` (`KismetMathLibrary.MakeVector2D` (`/Game/Source/MapSystem/Widgets/W_WorldMap.PlayerSizeX` _mapref) (`/Game/Source/MapSystem/Widgets/W_WorldMap.PlayerSizeY` _mapref)))
      (`self.ShowMap` false)
      (`UserWidget.AddToViewport` (`self.WMainRef`) 0))
    (:`Is Not Valid`
      (`KismetSystemLibrary.PrintString` "MapSystem: Initialize player failed, player is not set."))))

(event `self.ReceiveTick`
  (params (DeltaSeconds :type "Float (single-precision)"))
  (`self.UpdatePlayerMapL:ocation`))

(fn `ConvertLocationToMapLocation`
  (params (Location :type "Vector Structure"))
  (returns (Out :type "Vector2D Structure"))
  (bind (_returnvalue_x _returnvalue_y) (`KismetMathLibrary.BreakVector` (`Actor.K2_GetActorLocation` (`self.UpperLeft`))))
  (return (`KismetMathLibrary.MakeVector2D` (`KismetMathLibrary.Abs` (- Location_X _returnvalue_x)) (`KismetMathLibrary.Abs` (- Location_Y _returnvalue_y)))))

(fn `GetMapHeight`
  (returns (Height :type "Float (double-precision)"))
  (bind _returnvalue_x (`KismetMathLibrary.BreakVector` (`Actor.K2_GetActorLocation` (`self.LowerRight`))))
  (bind _returnvalue_x_2 (`KismetMathLibrary.BreakVector` (`Actor.K2_GetActorLocation` (`self.UpperLeft`))))
  (return (`KismetMathLibrary.Abs` (- _returnvalue_x_2 _returnvalue_x))))

(fn `GetMapWidth`
  (returns (Width :type "Float (double-precision)"))
  (bind (_returnvalue_x _returnvalue_y) (`KismetMathLibrary.BreakVector` (`Actor.K2_GetActorLocation` (`self.LowerRight`))))
  (bind (_returnvalue_x_2 _returnvalue_y_2) (`KismetMathLibrary.BreakVector` (`Actor.K2_GetActorLocation` (`self.UpperLeft`))))
  (return (`KismetMathLibrary.Abs` (- _returnvalue_y_2 _returnvalue_y))))

(fn `MapLocationToWidgetLocation`
  (params (Location :type "Vector Structure") (WidgetSize :type "Vector2D Structure"))
  (returns (Out :type "Vector2D Structure"))
  (bind (_x _y) (`KismetMathLibrary.BreakVector2D` WidgetSize))
  (bind _mapref (`self.MapRef`))
  (bind _out (`self.ConvertLocationToMapLocation` Location))
  (bind _width (`self.GetMapWidth`))
  (bind _height (`self.GetMapHeight`))
  (bind (_x_2 _y_2) (`KismetMathLibrary.BreakVector2D` _out))
  (return (`KismetMathLibrary.MakeVector2D` (- (* (/ _y_2 _width) (`/Game/Source/MapSystem/Widgets/W_WorldMap.MapSizeY` _mapref)) (/ _y 2.0)) (- (* (/ _x_2 _height) (`/Game/Source/MapSystem/Widgets/W_WorldMap.MapSizeX` _mapref)) (/ _x 2.0)))))

(fn `ShowMap`
  (params (`Show?` :type Boolean))
  (bind _visable_ (`self.Visable?`))
  (if (!= `Show?` _visable_)
    (set `self.Visable?` `Show?`)
    (if _visable_
      (`Widget.SetVisibility` (`self.MapRef`) "Visible")
      (else
        (`Widget.SetVisibility` (`self.MapRef`) "Hidden")))))

(fn `ToggleVisibility`
  (`self.ShowMap` (not (`self.Visable?`))))

(fn `UpdatePlayerMapL:ocation`
  (bind _out (`self.MapLocationToWidgetLocation` (`Actor.K2_GetActorLocation` (`self.Player`)) (`self.OriginalPlayerSize`)))
  (`Widget.SetRenderTranslation` (`/Game/Source/MapSystem/Widgets/W_WorldMap.PlayerBox` (`self.MapRef`)) _out))